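; Enemy character that idles spinning or patrols points in loop or ping-pong order, and shoots the player on sight.
; A Tick-driven state machine, paused during waits, switches on PawnSensing: noise turns it toward the sound, sight requires player light exposure to outweigh relative distance.
; Shooting prints harmless suppressive shots, then opens a timed window where the next shot applies lethal damage.
; Losing the target after a retriggerable delay restores the default state.
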(event `self.ReceiveBeginPlay`
  ;[1 0.3137 0] Auto-Patrol if PatrolPoints are set
  (if (> (`KismetArrayLibrary.Array_Length` (`self.PatrolPoints`)) 0)
    (bind _output_get (set `self.State` "NewEnumerator1"))
    (set `self.DefaultState` _output_get)))

(event `self.ReceiveTick`
  (params (DeltaSeconds :type "Float (single-precision)"))
  ;[1 0 0.02491] State Machine
  (if (not (`self.IsWaiting`))
    (switch `/Game/Nahash/Blueprints/Enemy/E_EnemyStates` (`self.State`)
      (:`NewEnumerator0`
        (`self.StateMachine_Idle`))
      (:`NewEnumerator1`
        (`self.StateMachine_Patrol`))
      (:`NewEnumerator2`
        (`self.StateMachine_ShootPlayer`))
      (:`NewEnumerator4`
        (`self.StateMachine_Aware`)))))

(event `self.PawnSensing.OnSeePawn`
  (params (Pawn :type "Pawn Object Reference"))
  ;[0 1 0.378] Detect Player
  (bind _asbp_first_person_character (cast `/Game/FirstPerson/Blueprints/BP_FirstPersonCharacter` Pawn))
  (bind _output_get (set `self.Target` _asbp_first_person_character))
  ;;[1 1 1 0.33] Lighting Exposition
  (if (> (`KismetMathLibrary.FMax` (`self.MinLightingPerception`) (`/Game/FirstPerson/Blueprints/BP_FirstPersonCharacter.lightExposition` _output_get)) (/ (`KismetMathLibrary.Vector_Distance` (`SceneComponent.K2_GetComponentLocation` (`Character.CapsuleComponent` _output_get)) (`SceneComponent.K2_GetComponentLocation` (`self.CapsuleComponent`))) (`PawnSensingComponent.SightRadius` (`self.PawnSensing`))))
    ;;[1 1 1 0.33] Start Shooting State
    (`|ExecutionSequence`
      (:`then_0`
        ;;;[1 1 1 0.33] Reset Movement if Entering State
        (if (`|EnumInequality` (`self.State`) "NewEnumerator2")
          (`NavMovementComponent.StopActiveMovement` (`self.CharacterMovement`))
          ;;;[1 1 1 0.33] Delay First Shoot
          (set `self.CanShoot` false)
          (`KismetSystemLibrary.Delay` (`self.StartShootDelay`))
          (set `self.CanShoot` true)))
      (:`then_1`
        (set `self.State` "NewEnumerator2")
        ;;[1 1 1 0.33] Unsee After Delay
        (`KismetSystemLibrary.RetriggerableDelay` (`self.UnseeAfterDelay`))
        (set `self.Target` null)))))

(event `StateMachine_Idle`
  ;[0 0.197 1] StateMachine: Idle
  ;;[1 1 1] Spin
  (`SceneComponent.K2_AddLocalRotation` (`self.CapsuleComponent`) (`KismetMathLibrary.MakeRotator` 0.0 0.0 (* (stale `self.ReceiveTick` DeltaSeconds) (`self.RotationSpeed`))) false false))

(event `StateMachine_Patrol`
  (bind _patrolpointid (`self.PatrolPointID`))
  ;[1 0.3137 0] StateMachine: Patrol
  ;;[1 1 1 0.33] Move To Next Point
  (`|AIMoveTo` self (0.0 0.0 0.0) (`|GetArrayItem` (`self.PatrolPoints`) (`self.PatrolPointID`)) 3.0
    (:`OnSuccess`
      ;;[1 1 1 0.33] Find Next Point
      (switch `/Game/Nahash/Blueprints/Enemy/E_PatrolType` (`self.PatrolType`)
        (:`NewEnumerator0`
          ;;;[1 1 1 0.33] Loop
          (set `self.PatrolPointID` (mod (+ (`self.PatrolPointID`) 1) (`KismetArrayLibrary.Array_Length` (`self.PatrolPoints`)))))
        (:`NewEnumerator1`
          ;;;[1 1 1 0.33] Ping-Pong
          (if (`self.IsPatrolingReverse`)
            (bind _result (`/Engine/EditorBlueprintResources/StandardMacros.DecrementInt` _patrolpointid)
              (:`  `
                (if (== _result 0)
                  (set `self.IsPatrolingReverse` (not (`self.IsPatrolingReverse`)) :!label _label))))
            (else
              (bind _result_2 (`/Engine/EditorBlueprintResources/StandardMacros.IncrementInt` _patrolpointid)
                (:`  `
                  (if (== _result_2 (- (`KismetArrayLibrary.Array_Length` (`self.PatrolPoints`)) 1))
                    (goto _label)
                    (else
                      _))))))))
      (`self.WaitFor` (`self.PatrolDelayPerPoint`)))))

(event `self.PawnSensing.OnHearNoise`
  (params (Instigator :type "Pawn Object Reference") (Location :type "Vector Structure (by ref)") (Volume :type "Float (single-precision)"))
  ;[0 0.6784 1] Hear Aware
  ;;[1 1 1 0.33] Check not Shooting
  (if (`|EnumInequality` (`self.State`) "NewEnumerator2")
    (set `self.AwareLocation` Location)
    (`|ExecutionSequence`
      (:`then_0`
        ;;[1 1 1 0.33] Reset Movement if Entering State
        (if (`|EnumInequality` (`self.State`) "NewEnumerator4")
          (`NavMovementComponent.StopActiveMovement` (`self.CharacterMovement`))))
      (:`then_1`
        (set `self.State` "NewEnumerator4")))))

(event `StateMachine_ShootPlayer`
  (bind _target (`self.Target`))
  ;[0 1 0.378] StateMachine: ShootPlayer
  (`/Engine/EditorBlueprintResources/StandardMacros.IsValid` _target
    (:`Is Valid`
      ;;[1 1 1 0.33] Look At Player
      (`self.Look At` (`SceneComponent.K2_GetComponentLocation` (`Actor.RootComponent` _target)) (stale `self.ReceiveTick` DeltaSeconds))
      (if (`self.CanShoot`)
        (`KismetSystemLibrary.PrintString` "SHOOT")
        (set `self.CanShoot` false)
        (bind _result (`/Engine/EditorBlueprintResources/StandardMacros.IncrementInt` (`self.CurrentShootTimes`))
          (:`  `
            (if (`self.ShouldNextShootKill`)
              ;;[1 1 1 0.33] Kill Target
              (`GameplayStatics.ApplyDamage` (`self.Target`) 1000.0 null self)
              (`KismetSystemLibrary.PrintString` "dead")
              (else
                ;;[1 1 1 0.33] Delay Next Shoot
                (if (== (+ _result 1) (`self.ShootTimes`))
                  (`KismetSystemLibrary.Delay` (`self.DeathShootDelay`))
                  (`|ExecutionSequence`
                    (:`then_0`
                      (set `self.CanShoot` true :!label _label_2))
                    (:`then_1`
                      ;;;[1 1 1 0.33] Next Shoot Kill Delay
                      (set `self.ShouldNextShootKill` true)
                      (`KismetSystemLibrary.RetriggerableDelay` (`self.InstantShootLifeTime`))
                      (set `self.ShouldNextShootKill` false)
                      (set `self.CurrentShootTimes` 0)
                      (`KismetSystemLibrary.PrintString` "reset ammo")))
                  (else
                    (`KismetSystemLibrary.Delay` (`self.SupressShootDelay`))
                    (goto _label_2)))))))))
    (:`Is Not Valid`
      ;;[1 1 1 0.33] Fallback to Default State
      (set `self.State` (`self.DefaultState`))
      (`self.WaitFor` (`self.TimeAfterShootEndToDefaultState`)))))

(event `StateMachine_Aware`
  ;[0 0.6784 1] StateMachine: Aware
  (`self.Look At` (`self.AwareLocation`) (stale `self.ReceiveTick` DeltaSeconds))
  (`KismetSystemLibrary.PrintString` "aware"))

(fn `Look At`
  (params (Target :type "Vector Structure") (`Delta Time` :type "Float (double-precision)"))
  (bind _capsulecomponent (`self.CapsuleComponent`))
  (`SceneComponent.K2_SetWorldRotation` _capsulecomponent (`KismetMathLibrary.RInterpTo` (`SceneComponent.K2_GetComponentRotation` _capsulecomponent) (`KismetMathLibrary.MakeRotator` 0.0 0.0 (.yaw (`KismetMathLibrary.FindLookAtRotation` (`SceneComponent.K2_GetComponentLocation` _capsulecomponent) Target))) `Delta Time` (`self.RotationSpeed`)) false false))

(fn `UserConstructionScript`)