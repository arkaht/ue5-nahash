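; Enemy character that idles, patrols, or turns to face the player when spotted.
; A Tick-driven state machine spins in Idle, follows patrol points via AIMoveTo in loop or ping-pong order, and rotates toward the target in ShootPlayer, which fires nothing itself.
; PawnSensing sets the target, and a retriggerable delay clears it when sightings stop, restoring the default state.
; WaitFor pauses the state machine after patrol points and lost targets.
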(event `self.ReceiveBeginPlay`
  ;[1 0.3137 0] Auto-Patrol if PatrolPoints are set
  (if (> (`KismetArrayLibrary.Array_Length` (`self.PatrolPoints`)) 0)
    (bind _output_get (set `self.State` "NewEnumerator1"))
    (set `self.DefaultState` _output_get)))

(event `self.ReceiveTick`
  (params (DeltaSeconds :type "Float (single-precision)"))
  ;[1 0 0.02491] State Machine
  (if (not (`self.IsWaiting`))
    (switch `/Game/Nahash/Blueprints/E_EnemyStates` (`self.State`)
      (:`NewEnumerator0`
        (`self.StateMachine_Idle`))
      (:`NewEnumerator1`
        (`self.StateMachine_Patrol`))
      (:`NewEnumerator2`
        (`self.StateMachine_ShootPlayer`)))))

(event `self.PawnSensing.OnSeePawn`
  (params (Pawn :type "Pawn Object Reference"))
  ;[0 1 0.378] Detect Player
  (bind _asbp_first_person_character (cast `/Game/FirstPerson/Blueprints/BP_FirstPersonCharacter` Pawn))
  (set `self.Target` _asbp_first_person_character)
  ;;[1 1 1 0.33] Start Shooting State
  (`|ExecutionSequence`
    (:`then_0`
      ;;;[1 1 1 0.33] Reset Movement if Entering State
      (if (`|EnumInequality` (`self.State`) "NewEnumerator2")
        (`NavMovementComponent.StopActiveMovement` (`self.CharacterMovement`))))
    (:`then_1`
      (set `self.State` "NewEnumerator2")
      ;;[1 1 1 0.33] Unsee After Delay
      (`KismetSystemLibrary.RetriggerableDelay` 0.6)
      (set `self.Target` null))))

(event `StateMachine_Idle`
  ;[0 0.197 1] StateMachine: Idle
  ;;[1 1 1] Spin
  (`SceneComponent.K2_AddLocalRotation` (`self.CapsuleComponent`) (`KismetMathLibrary.MakeRotator` 0.0 0.0 (* (stale `self.ReceiveTick` DeltaSeconds) (`self.RotationSpeed`))) false false))

(event `StateMachine_Patrol`
  (bind _patrolpointid (`self.PatrolPointID`))
  ;[1 0.3137 0] StateMachine: Patrol
  ;;[1 1 1 0.33] Move To Next Point
  (`|AIMoveTo` self (0.0 0.0 0.0) (`|GetArrayItem` (`self.PatrolPoints`) (`self.PatrolPointID`)) 3.0
    (:`OnSuccess`
      ;;[1 1 1 0.33] Find Next Point
      (switch `/Game/Nahash/Blueprints/E_PatrolType` (`self.PatrolType`)
        (:`NewEnumerator0`
          ;;;[1 1 1 0.33] Loop
          (set `self.PatrolPointID` (mod (+ (`self.PatrolPointID`) 1) (`KismetArrayLibrary.Array_Length` (`self.PatrolPoints`)))))
        (:`NewEnumerator1`
          ;;;[1 1 1 0.33] Ping-Pong
          (if (`self.IsPatrolingReverse`)
            (bind _output_get (set `self.PatrolPointID` (- _patrolpointid 1)))
            (if (== _output_get 0)
              (set `self.IsPatrolingReverse` (not (`self.IsPatrolingReverse`)) :!label _label))
            (else
              (bind _output_get_2 (set `self.PatrolPointID` (+ _patrolpointid 1)))
              (if (== _output_get_2 (- (`KismetArrayLibrary.Array_Length` (`self.PatrolPoints`)) 1))
                (goto _label)
                (else
                  _))))))
      (`self.WaitFor` (`self.PatrolDelayPerPoint`)))))

(event `StateMachine_ShootPlayer`
  (bind _target (`self.Target`))
  (bind _capsulecomponent (`self.CapsuleComponent`))
  ;[0 1 0.378] StateMachine: ShootPlayer
  (`/Engine/EditorBlueprintResources/StandardMacros.IsValid` _target
    (:`Is Valid`
      ;;[1 1 1 0.33] Look At Player
      (`SceneComponent.K2_SetWorldRotation` _capsulecomponent (`KismetMathLibrary.RInterpTo` (`SceneComponent.K2_GetComponentRotation` _capsulecomponent) (`KismetMathLibrary.MakeRotator` 0.0 0.0 (.yaw (`KismetMathLibrary.FindLookAtRotation` (`SceneComponent.K2_GetComponentLocation` _capsulecomponent) (`SceneComponent.K2_GetComponentLocation` (`Actor.RootComponent` _target))))) (stale `self.ReceiveTick` DeltaSeconds) (`self.RotationSpeed`)) false false))
    (:`Is Not Valid`
      ;;[1 1 1 0.33] Fallback to Default State
      (set `self.State` (`self.DefaultState`))
      (`self.WaitFor` (`self.TimeAfterShootEndToDefaultState`)))))

(fn `UserConstructionScript`)