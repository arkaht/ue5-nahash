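; BP_LightSpot is a breakable spot light that reports how exposed the first-person player is to its light.
; Entering its sphere adds an entry to the player's LightExpositions array and stores the index; leaving removes it.
; While registered, Tick line traces to the player and, on a hit, updates that entry from distance through RangeCurve.
; Destroy hides the light, plays breaking glass, disables overlaps and removes any active entry.
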(event `self.Sphere.OnComponentBeginOverlap`
  (params (OverlappedComponent :type "PrimitiveComponent Object Reference") (OtherActor :type "Actor Object Reference") (OtherComp :type "PrimitiveComponent Object Reference") (OtherBodyIndex :type Integer) (bFromSweep :type Boolean) (SweepResult :type "HitResult Structure (by ref)"))
  (bind _asbp_first_person_character (cast `/Game/FirstPerson/Blueprints/BP_FirstPersonCharacter` OtherActor))
  (bind _output_get (set `self.player` _asbp_first_person_character))
  (bind _returnvalue (`KismetArrayLibrary.Array_Add` (`/Game/FirstPerson/Blueprints/BP_FirstPersonCharacter.lightExpositions` _output_get) (`self.lightExposition`)))
  (set `self.indexInPlayerArray` _returnvalue))

(event `self.Sphere.OnComponentEndOverlap`
  (params (OverlappedComponent :type "PrimitiveComponent Object Reference") (OtherActor :type "Actor Object Reference") (OtherComp :type "PrimitiveComponent Object Reference") (OtherBodyIndex :type Integer))
  (bind _asbp_first_person_character (cast `/Game/FirstPerson/Blueprints/BP_FirstPersonCharacter` OtherActor))
  (`KismetArrayLibrary.Array_Remove` (`/Game/FirstPerson/Blueprints/BP_FirstPersonCharacter.lightExpositions` _asbp_first_person_character) (`self.indexInPlayerArray`))
  (set `self.lightExposition` 0.0)
  (set `self.indexInPlayerArray` -1))

(event `self.ReceiveTick`
  (params (DeltaSeconds :type "Float (single-precision)"))
  (if (!= (`self.indexInPlayerArray`) -1)
    (bind _outhit (`KismetSystemLibrary.LineTraceSingleForObjects` (`SceneComponent.K2_GetComponentLocation` (`self.SpotLight`)) (`SceneComponent.K2_GetComponentLocation` (`Actor.RootComponent` (`self.player`))) (`|MakeArray` "ObjectTypeQuery1" "ObjectTypeQuery2" "ObjectTypeQuery3" :!type "EObjectTypeQuery Enum")))
    (cast `/Game/FirstPerson/Blueprints/BP_FirstPersonCharacter` (`.HitActor` (`GameplayStatics.BreakHitResult` _outhit)))
    (bind _output_get (set `self.lightExposition` (`CurveFloat.GetFloatValue` (`self.rangeCurve`) (`KismetMathLibrary.NormalizeToRange` (`self.GetDistanceTo` (`self.player`)) 0.0 500.0))))
    (`KismetArrayLibrary.Array_Set` (`/Game/FirstPerson/Blueprints/BP_FirstPersonCharacter.lightExpositions` (`self.player`)) (`self.indexInPlayerArray`) _output_get)))

(fn `Destroy`
  (set `self.destroyed` true)
  (`SceneComponent.SetVisibility` (`self.SpotLight`) false false)
  (`GameplayStatics.PlaySoundAtLocation` "/Game/SFX/SC_BrokenGlass.SC_BrokenGlass" (`SceneComponent.K2_GetComponentLocation` (`self.SpotLight`)) (struct) 1.0 1.0 0.0 null null null null)
  (set `PrimitiveComponent.bGenerateOverlapEvents` false (`self.Sphere`))
  (`ActorComponent.K2_DestroyComponent` (`self.Sphere1`))
  (if (!= (`self.indexInPlayerArray`) -1)
    (`KismetArrayLibrary.Array_Remove` (`/Game/FirstPerson/Blueprints/BP_FirstPersonCharacter.lightExpositions` (`self.player`)) (`self.indexInPlayerArray`))
    (set `self.lightExposition` 0.0)
    (set `self.indexInPlayerArray` -1)))

(fn `UserConstructionScript`)